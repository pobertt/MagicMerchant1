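; BP_TestCollectable is a test collectable that adds its Inventory data to the player's inventory.
; Its AddInventory event first calls EnemyKilled on the player, then passes the data to the player's Comp_Inventory.
; On success it finds the first top-level WBP_Inventory widget, rebuilds its grid through SetGrid and prints a confirmation if that widget is valid.
; On failure it prints that the inventory is full.
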(event Custom|AddInventory
  (bind _playerref (Variables|Default|GetPlayerRef))
  (Class|BetterPlayerCharacter|EnemyKilled _playerref)
  (bind _itemadded (Default|AddtoInventory (Actor|GetComponentbyClass _playerref "/Game/Inventory/Comp_Inventory.Comp_Inventory_C") (Variables|Default|GetInventory)))
  (if _itemadded
    (bind _foundwidgets (Widget|GetAllWidgetsOfClass "/Game/Inventory/WBP_Inventory.WBP_Inventory_C" true))
    (Utilities|IsValid (Utilities|Array|Get(acopy) _foundwidgets)
      (:Is%20Valid
        (Default|SetGrid (Utilities|Array|Get(acopy) _foundwidgets))
        (Development|PrintString "Item Added")))
    (else
      (Development|PrintString "inventory full"))))

(fn ConstructionScript)