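; BP_Player is a player Blueprint that acts as a test harness for player stats and currencies.
; On BeginPlay it enables input from the first player controller, then creates a WBP_UI widget and stores it, without adding it to the viewport here.
; Debug numpad keys call functions that add HP, MP, money, a second currency and levels, with the money result printed on screen.
; A separate SayHey event prints a greeting.
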(event EventBeginPlay
  (bind _returnvalue (Game|GetPlayerController 0))
  ;[1 1 1] Player Controller
  (Input|EnableInput _returnvalue)
  (bind _returnvalue_2 (UserInterface|CreateWidget "/Game/WBP_UI.WBP_UI_C" _returnvalue))
  (Variables|Default|SetUIBP _returnvalue_2))

(event Collision|EventActorBeginOverlap
  (params (OtherActor :type Actor%20Object%20Reference)))

(event EventTick
  (params (DeltaSeconds :type Float%20%28single-precision%29)))

(event EventSayHey
  (Development|PrintString "Hey"))

(event Input|KeyboardEvents|NumPadThree
  (params (Key :type Key%20Structure :default "None"))
  ;[1 1 1] Debug Adding to Stats
  (:Pressed
    (bind _returnvalue (Class|PlayerCharacter|AddMoney))
    (Development|PrintString (Utilities|String|ToString(Float) _returnvalue))))

(event Input|KeyboardEvents|NumPadOne
  (params (Key :type Key%20Structure :default "None"))
  ;[1 1 1] Debug Adding to Stats
  (:Pressed
    (Class|PlayerCharacter|AddHp)))

(event Input|KeyboardEvents|NumPadTwo
  (params (Key :type Key%20Structure :default "None"))
  ;[1 1 1] Debug Adding to Stats
  (:Pressed
    (Class|PlayerCharacter|AddMp)))

(event Input|KeyboardEvents|NumPadFour
  (params (Key :type Key%20Structure :default "None"))
  ;[1 1 1] Debug Adding to Stats
  (:Pressed
    (Class|PlayerCharacter|AddCurrency2)))

(event Input|KeyboardEvents|NumPadFive
  (params (Key :type Key%20Structure :default "None"))
  ;[1 1 1] Debug Adding to Stats
  (:Pressed
    (Class|PlayerCharacter|AddLvl)))

(fn ConstructionScript)