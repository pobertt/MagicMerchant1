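; Player character Blueprint that registers the main UI with the game mode on BeginPlay and handles player death.
; Debug number keys and input actions add or subtract HP, MP, money, a second currency and level.
; The C key flip-flops between the game mode's combat widget and a freshly created main UI widget.
; On death it loads a quit level instance, shows a game-over widget and pauses the game.
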(event Collision|EventActorBeginOverlap
  (params (OtherActor :type Actor%20Object%20Reference)))

(event EventPlayerDead
  (Class|LevelStreamingDynamic|LoadLevelInstance "QuitLevel" "0, 0, 0" "0, 0, 0" "" 0 false)
  (Development|PrintString "I should die now")
  (bind _returnvalue (UserInterface|CreateWidget "/Game/UserInterface/WBP_GameOver.WBP_GameOver_C"))
  (UserInterface|Viewport|AddtoViewport _returnvalue 0)
  (Game|SetGamePaused true))

(event EventBeginPlay
  ;[1 1 1] Player Controller
  (bind _asmy_magic_merchant_1game_mode_base (Utilities|Casting|CastToMyMagicMerchant1GameModeBase (Game|GetGameMode)))
  (bind _output_get (Variables|Default|SetGameModeRef _asmy_magic_merchant_1game_mode_base))
  (Class|MagicMerchant1GameModeBase|AddMainUIWidget _output_get))

(event Input|ActionEvents|InputActionSubtractHP
  (params (Key :type Key%20Structure :default "None"))
  ;[1 1 1] Debugging Subtracting to Stats
  (:Pressed
    (Class|BetterPlayerCharacter|SubHp)))

(event Input|ActionEvents|InputActionSubtractMP
  (params (Key :type Key%20Structure :default "None"))
  ;[1 1 1] Debugging Subtracting to Stats
  (:Pressed
    (Class|BetterPlayerCharacter|SubMp 0.0)))

(event Input|ActionEvents|InputActionSubtractMoney
  (params (Key :type Key%20Structure :default "None"))
  ;[1 1 1] Debugging Subtracting to Stats
  (:Pressed
    (Class|BetterPlayerCharacter|SubMoney)))

(event Input|ActionEvents|InputActionSubtractCurrency2
  (params (Key :type Key%20Structure :default "None"))
  ;[1 1 1] Debugging Subtracting to Stats
  (:Pressed
    (Class|BetterPlayerCharacter|SubCurrency2)))

(event Input|ActionEvents|InputActionSubtractLevel
  (params (Key :type Key%20Structure :default "None"))
  ;[1 1 1] Debugging Subtracting to Stats
  (:Pressed
    (Class|BetterPlayerCharacter|SubLvl)))

(event Input|KeyboardEvents|1
  (params (Key :type Key%20Structure :default "None"))
  ;[1 1 1] Debug Adding to Stats
  (:Pressed
    (Class|BetterPlayerCharacter|AddHp 1.0)))

(event Input|KeyboardEvents|C
  (params (Key :type Key%20Structure :default "None"))
  (bind _gamemoderef (Variables|Default|GetGameModeRef))
  ;[1 1 1] Adding/Removing Combat Widget Viewport
  (:Pressed
    (Utilities|FlowControl|FlipFlop
      (:A
        (Viewport|RemoveAllWidgets)
        (Class|MagicMerchant1GameModeBase|AddCombatWidget _gamemoderef))
      (:B
        (Class|MagicMerchant1GameModeBase|RemoveCombatWidget _gamemoderef)
        (bind _returnvalue (UserInterface|CreateWidget "/Game/UserInterface/WBP_UI.WBP_UI_C" (Game|GetPlayerController 0)))
        (UserInterface|Viewport|AddtoViewport _returnvalue 0)))))

(event Input|KeyboardEvents|3
  (params (Key :type Key%20Structure :default "None"))
  ;[1 1 1] Debug Adding to Stats
  (:Pressed
    (Class|BetterPlayerCharacter|AddMoney 1.0)))

(event Input|KeyboardEvents|2
  (params (Key :type Key%20Structure :default "None"))
  ;[1 1 1] Debug Adding to Stats
  (:Pressed
    (Class|BetterPlayerCharacter|AddMp 0.0)))

(event Input|KeyboardEvents|4
  (params (Key :type Key%20Structure :default "None"))
  ;[1 1 1] Debug Adding to Stats
  (:Pressed
    (Class|BetterPlayerCharacter|AddCurrency2)))

(event Input|KeyboardEvents|5
  (params (Key :type Key%20Structure :default "None"))
  ;[1 1 1] Debug Adding to Stats
  (:Pressed
    (Class|BetterPlayerCharacter|AddLvl)))

(fn ConstructionScript)